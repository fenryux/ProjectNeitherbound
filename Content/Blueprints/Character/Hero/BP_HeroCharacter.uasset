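; Player hero character Blueprint that handles camera-relative movement and spring arm camera zoom through Enhanced Input.
; On BeginPlay it sets the player controller's control rotation to the spring arm's target rotation.
; IA_Move feeds movement input along the control rotation's forward and right vectors.
; IA_CameraZoom sets the spring arm length directly from the scaled input value, clamped to ZoomBounds, rather than offsetting the current length.
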(event `self.ReceiveBeginPlay`
  ;[1 1 1] Set Character rotation to Camera rotation
  (`Controller.SetControlRotation` (`GameplayStatics.GetPlayerController` 0) (`SpringArmComponent.GetTargetRotation` (`self.SpringArm`))))

(event `EnhancedInput|/Game/Blueprints/Input/InputActions/IA_CameraZoom`
  (params (ActionValue :type "Float (double-precision)") (ElapsedSeconds :type "Float (double-precision)") (TriggeredSeconds :type "Float (double-precision)") (InputAction :type "InputAction Object Reference" :default "/Game/Blueprints/Input/InputActions/IA_CameraZoom.IA_CameraZoom"))
  (bind (_x _y) (`KismetMathLibrary.BreakVector2D` (`self.ZoomBounds`)))
  ;[1 1 1] Camera Zoom with Mouse input
  (:`Triggered`
    (set `SpringArmComponent.TargetArmLength` (`KismetMathLibrary.FClamp` (+ (* ActionValue (`self.ZoomMultiplier`)) 0.0) _x _y) (`self.SpringArm`))))

(event `EnhancedInput|/Game/Blueprints/Input/InputActions/IA_Move`
  (params (ActionValue :type "Vector2D Structure") (ElapsedSeconds :type "Float (double-precision)") (TriggeredSeconds :type "Float (double-precision)") (InputAction :type "InputAction Object Reference" :default "/Game/Blueprints/Input/InputActions/IA_Move.IA_Move"))
  (bind (_x _y) (`KismetMathLibrary.BreakVector2D` ActionValue))
  (bind _returnvalue (`self.GetControlRotation`))
  ;[1 1 1] Character Movement handling
  (:`Triggered`
    (`self.AddMovementInput` (`KismetMathLibrary.GetForwardVector` _returnvalue) _y)
    (`self.AddMovementInput` (`KismetMathLibrary.GetRightVector` _returnvalue) _x)))

(fn `UserConstructionScript`)